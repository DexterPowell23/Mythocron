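; Test dummy Blueprint that reacts to hits from the ThirdPersonCharacter based on which side is struck.
; Front, Back, Left and Right components check on begin overlap whether they touch the character's HIt component.
; A hit plays a one-shot animation and prints "hit", while other character overlaps play the looping dummy animation.
; Left and Right play the opposite-named animations, and Front's hit branch has no animation assigned.
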(event `self.Front.OnComponentBeginOverlap`
  (params (OverlappedComponent :type "PrimitiveComponent Object Reference") (OtherActor :type "Actor Object Reference") (OtherComp :type "PrimitiveComponent Object Reference") (OtherBodyIndex :type Integer) (bFromSweep :type Boolean) (SweepResult :type "HitResult Structure (by ref)"))
  (bind _mesh (`self.Mesh`))
  (bind _asthird_person_character (cast `/Game/ThirdPersonBP/Blueprints/ThirdPersonCharacter` OtherActor))
  (if (`PrimitiveComponent.IsOverlappingComponent` (`self.Front`) (`/Game/ThirdPersonBP/Blueprints/ThirdPersonCharacter.HIt` _asthird_person_character))
    (`SkeletalMeshComponent.PlayAnimation` _mesh null false)
    (`KismetSystemLibrary.PrintString` "hit" :!label _label)
    (else
      (`SkeletalMeshComponent.PlayAnimation` _mesh "/Game/Project_mythocron/Animation/Dummy/SK_Dummy_Loop.SK_Dummy_Loop" true))))

(event `self.Back.OnComponentBeginOverlap`
  (params (OverlappedComponent :type "PrimitiveComponent Object Reference") (OtherActor :type "Actor Object Reference") (OtherComp :type "PrimitiveComponent Object Reference") (OtherBodyIndex :type Integer) (bFromSweep :type Boolean) (SweepResult :type "HitResult Structure (by ref)"))
  (bind _mesh (`self.Mesh`))
  (bind _asthird_person_character (cast `/Game/ThirdPersonBP/Blueprints/ThirdPersonCharacter` OtherActor))
  (if (`PrimitiveComponent.IsOverlappingComponent` (`self.Back`) (`/Game/ThirdPersonBP/Blueprints/ThirdPersonCharacter.HIt` _asthird_person_character))
    (`SkeletalMeshComponent.PlayAnimation` _mesh "/Game/Project_mythocron/Animation/Dummy/SK_Dummy_Back.SK_Dummy_Back" false)
    (goto _label)
    (else
      (`SkeletalMeshComponent.PlayAnimation` _mesh "/Game/Project_mythocron/Animation/Dummy/SK_Dummy_Loop.SK_Dummy_Loop" true))))

(event `self.Right.OnComponentBeginOverlap`
  (params (OverlappedComponent :type "PrimitiveComponent Object Reference") (OtherActor :type "Actor Object Reference") (OtherComp :type "PrimitiveComponent Object Reference") (OtherBodyIndex :type Integer) (bFromSweep :type Boolean) (SweepResult :type "HitResult Structure (by ref)"))
  (bind _mesh (`self.Mesh`))
  (bind _asthird_person_character (cast `/Game/ThirdPersonBP/Blueprints/ThirdPersonCharacter` OtherActor))
  (if (`PrimitiveComponent.IsOverlappingComponent` (`self.Right`) (`/Game/ThirdPersonBP/Blueprints/ThirdPersonCharacter.HIt` _asthird_person_character))
    (`SkeletalMeshComponent.PlayAnimation` _mesh "/Game/Project_mythocron/Animation/Dummy/SK_Dummy_Left.SK_Dummy_Left" false)
    (goto _label)
    (else
      (`SkeletalMeshComponent.PlayAnimation` _mesh "/Game/Project_mythocron/Animation/Dummy/SK_Dummy_Loop.SK_Dummy_Loop" true))))

(event `self.Left.OnComponentBeginOverlap`
  (params (OverlappedComponent :type "PrimitiveComponent Object Reference") (OtherActor :type "Actor Object Reference") (OtherComp :type "PrimitiveComponent Object Reference") (OtherBodyIndex :type Integer) (bFromSweep :type Boolean) (SweepResult :type "HitResult Structure (by ref)"))
  (bind _mesh (`self.Mesh`))
  (bind _asthird_person_character (cast `/Game/ThirdPersonBP/Blueprints/ThirdPersonCharacter` OtherActor))
  (if (`PrimitiveComponent.IsOverlappingComponent` (`self.Left`) (`/Game/ThirdPersonBP/Blueprints/ThirdPersonCharacter.HIt` _asthird_person_character))
    (`SkeletalMeshComponent.PlayAnimation` _mesh "/Game/Project_mythocron/Animation/Dummy/SK_Dummy_Right.SK_Dummy_Right" false)
    (goto _label)
    (else
      (`SkeletalMeshComponent.PlayAnimation` _mesh "/Game/Project_mythocron/Animation/Dummy/SK_Dummy_Loop.SK_Dummy_Loop" true))))

(fn `UserConstructionScript`)