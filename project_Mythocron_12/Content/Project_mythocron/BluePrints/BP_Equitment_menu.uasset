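; BP_Equitment_menu is a trigger actor that opens an equipment menu when the ThirdPersonCharacter enters its box.
; Overlap switches to the character's FollowCamera1, disables input, teleports it to a hard-coded spot, and shows a W_Equitment widget with the mouse cursor.
; The widget receives a reference to this actor, whose quit event restores camera and input and removes the menu.
; A DoOnce, reset when the character leaves the box, guards against repeated opening.
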(event `self.Box.OnComponentBeginOverlap`
  (params (OverlappedComponent :type "PrimitiveComponent Object Reference") (OtherActor :type "Actor Object Reference") (OtherComp :type "PrimitiveComponent Object Reference") (OtherBodyIndex :type Integer) (bFromSweep :type Boolean) (SweepResult :type "HitResult Structure (by ref)"))
  (bind _returnvalue (`GameplayStatics.GetPlayerController` 0))
  (`/Engine/EditorBlueprintResources/StandardMacros.DoOnce` false :!label _label
    (:`Completed`
      (`self.Equit`
        (:`then`)
        (:`else`
          (bind _asthird_person_character (cast `/Game/ThirdPersonBP/Blueprints/ThirdPersonCharacter` OtherActor))
          (`ActorComponent.SetActive` (`/Game/ThirdPersonBP/Blueprints/ThirdPersonCharacter.FollowCamera1` _asthird_person_character) true false)
          (`ActorComponent.SetActive` (`/Game/ThirdPersonBP/Blueprints/ThirdPersonCharacter.FollowCamera` _asthird_person_character) false false)
          (`self.DisableInput` _returnvalue _returnvalue)
          (`self.DisableInput` _asthird_person_character _returnvalue)
          (`self.K2_TeleportTo` _asthird_person_character (-790.0 2830.0 770.720947) (struct :`Yaw` 170.0))
          (bind _returnvalue_2 (`|CreateWidget` "/Game/Project_mythocron/widget/W_Equitment.W_Equitment_C" null self))
          (bind _output_get (set `self.Equit` _returnvalue_2))
          (`UserWidget.AddToViewport` _output_get 0)
          (set `PlayerController.bShowMouseCursor` true _returnvalue))))))

(event `self.Box.OnComponentEndOverlap`
  (params (OverlappedComponent :type "PrimitiveComponent Object Reference") (OtherActor :type "Actor Object Reference") (OtherComp :type "PrimitiveComponent Object Reference") (OtherBodyIndex :type Integer))
  (cast `/Game/ThirdPersonBP/Blueprints/ThirdPersonCharacter` OtherActor)
  (goto _label :!via `Reset`))

(event `quit`
  (bind _returnvalue (`GameplayStatics.GetPlayerController` 0))
  (`self.Equit`
    (:`then`
      (bind _asthird_person_character (cast `/Game/ThirdPersonBP/Blueprints/ThirdPersonCharacter` (`GameplayStatics.GetPlayerCharacter` 0)))
      (`ActorComponent.SetActive` (`/Game/ThirdPersonBP/Blueprints/ThirdPersonCharacter.FollowCamera1` _asthird_person_character) false false)
      (`ActorComponent.SetActive` (`/Game/ThirdPersonBP/Blueprints/ThirdPersonCharacter.FollowCamera` _asthird_person_character) true false)
      (`self.EnableInput` _returnvalue _returnvalue)
      (`self.EnableInput` _asthird_person_character _returnvalue)
      (`Widget.RemoveFromParent` (`self.Equit`))
      (set `PlayerController.bShowMouseCursor` false _returnvalue))
    (:`else`)))

(fn `UserConstructionScript`)