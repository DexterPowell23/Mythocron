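; BP_Dumb_test is a test actor that plays directional hit reactions when struck by the ThirdPersonCharacter.
; Front, Back, Right and Left components handle begin-overlap, cast the other actor and check overlap with its HIt component.
; A match plays a one-shot animation on Mesh, otherwise a looping one.
; Left reuses the right reaction, and Right falls back to the left animation instead of the common loop.
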(event `self.Front.OnComponentBeginOverlap`
  (params (OverlappedComponent :type "PrimitiveComponent Object Reference") (OtherActor :type "Actor Object Reference") (OtherComp :type "PrimitiveComponent Object Reference") (OtherBodyIndex :type Integer) (bFromSweep :type Boolean) (SweepResult :type "HitResult Structure (by ref)"))
  (bind _mesh (`self.Mesh`))
  (bind _asthird_person_character (cast `/Game/ThirdPersonBP/Blueprints/ThirdPersonCharacter` OtherActor))
  (if (`PrimitiveComponent.IsOverlappingComponent` (`self.Front`) (`/Game/ThirdPersonBP/Blueprints/ThirdPersonCharacter.HIt` _asthird_person_character))
    (`SkeletalMeshComponent.PlayAnimation` _mesh "/Game/Project_mythocron/Animation/Anim_Dumb_TestFront.Anim_Dumb_TestFront" false)
    (else
      (`SkeletalMeshComponent.PlayAnimation` _mesh "/Game/Project_mythocron/Animation/Anim_Dumb_Testloop.Anim_Dumb_Testloop" true))))

(event `self.Back.OnComponentBeginOverlap`
  (params (OverlappedComponent :type "PrimitiveComponent Object Reference") (OtherActor :type "Actor Object Reference") (OtherComp :type "PrimitiveComponent Object Reference") (OtherBodyIndex :type Integer) (bFromSweep :type Boolean) (SweepResult :type "HitResult Structure (by ref)"))
  (bind _mesh (`self.Mesh`))
  (bind _asthird_person_character (cast `/Game/ThirdPersonBP/Blueprints/ThirdPersonCharacter` OtherActor))
  (if (`PrimitiveComponent.IsOverlappingComponent` (`self.Back`) (`/Game/ThirdPersonBP/Blueprints/ThirdPersonCharacter.HIt` _asthird_person_character))
    (`SkeletalMeshComponent.PlayAnimation` _mesh "/Game/Project_mythocron/Animation/Anim_Dumb_Testback.Anim_Dumb_Testback" false)
    (else
      (`SkeletalMeshComponent.PlayAnimation` _mesh "/Game/Project_mythocron/Animation/Anim_Dumb_Testloop.Anim_Dumb_Testloop" true))))

(event `self.Right.OnComponentBeginOverlap`
  (params (OverlappedComponent :type "PrimitiveComponent Object Reference") (OtherActor :type "Actor Object Reference") (OtherComp :type "PrimitiveComponent Object Reference") (OtherBodyIndex :type Integer) (bFromSweep :type Boolean) (SweepResult :type "HitResult Structure (by ref)"))
  (bind _mesh (`self.Mesh`))
  (bind _asthird_person_character (cast `/Game/ThirdPersonBP/Blueprints/ThirdPersonCharacter` OtherActor))
  (if (`PrimitiveComponent.IsOverlappingComponent` (`self.Right`) (`/Game/ThirdPersonBP/Blueprints/ThirdPersonCharacter.HIt` _asthird_person_character))
    (`SkeletalMeshComponent.PlayAnimation` _mesh "/Game/Project_mythocron/Animation/Anim_Dumb_Testright.Anim_Dumb_Testright" false)
    (else
      (`SkeletalMeshComponent.PlayAnimation` _mesh "/Game/Project_mythocron/Animation/Anim_Dumb_TestLeft.Anim_Dumb_TestLeft" true))))

(event `self.Left.OnComponentBeginOverlap`
  (params (OverlappedComponent :type "PrimitiveComponent Object Reference") (OtherActor :type "Actor Object Reference") (OtherComp :type "PrimitiveComponent Object Reference") (OtherBodyIndex :type Integer) (bFromSweep :type Boolean) (SweepResult :type "HitResult Structure (by ref)"))
  (bind _mesh (`self.Mesh`))
  (bind _asthird_person_character (cast `/Game/ThirdPersonBP/Blueprints/ThirdPersonCharacter` OtherActor))
  (if (`PrimitiveComponent.IsOverlappingComponent` (`self.Left`) (`/Game/ThirdPersonBP/Blueprints/ThirdPersonCharacter.HIt` _asthird_person_character))
    (`SkeletalMeshComponent.PlayAnimation` _mesh "/Game/Project_mythocron/Animation/Anim_Dumb_Testright.Anim_Dumb_Testright" false)
    (else
      (`SkeletalMeshComponent.PlayAnimation` _mesh "/Game/Project_mythocron/Animation/Anim_Dumb_Testloop.Anim_Dumb_Testloop" true))))

(fn `UserConstructionScript`)